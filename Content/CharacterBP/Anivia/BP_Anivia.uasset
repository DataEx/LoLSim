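; Playable Anivia champion for top-down play, handling Q, W, E and R targeting, casting, cooldowns and HUD.
; Ability keys enter a setting state and cancel the others; AcceptAction commits, CancelAction backs out.
; W and R previews follow the flat cursor until placed; Q fires toward it, and re-pressing Q or R can end them.
; E launches a homing projectile, auto-pathing into range via Tick unless new movement input interrupts.
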(event Custom|SpawnAndTargetEAbility
  (params (SpawnLocation :type Vector) (SpawnRotation :type Rotator) (Target :type Primitive%20Component%20Object%20Reference))
  ;[1 1 1] Place abilities into world after spawn position has been decided upon
  (bind _returnvalue (Game|SpawnActorfromClass "/Game/AbilitiesBP/Anivia/AniviaE.AniviaE_C" (Math|Transform|MakeTransform SpawnLocation SpawnRotation "1,1,1") "Undefined" 0 0))
  (Variables|/Game/AbilitiesBP/Anivia/AniviaE.AniviaE_C|SetTarget _returnvalue Target)
  (Variables|/Script/Engine.ProjectileMovementComponent|SetHomingTargetComponent (Variables|/Game/AbilitiesBP/Anivia/AniviaE.AniviaE_C|GetProjectileMovement _returnvalue) Target)
  (Rendering|SetVisibility (Variables|Default|GetCircularAbilityRangeIndicator) false false)
  (Variables|Default|SetIsSettingE false)
  (Variables|Default|SetCanUseE false)
  (Default|ResetCooldownSwitcher (Variables|Default|GetHUD) "NewEnumerator2")
  (Utilities|FlowControl|Delay (Variables|Default|GetECooldown))
  (Variables|Default|SetCanUseE true))

(event Custom|FireQAbility
  (bind _abilityspawnpoint (Variables|Default|GetAbilitySpawnPoint))
  (bind _returnvalue (Transformation|GetWorldLocation _abilityspawnpoint))
  ;[1 1 1] Fire Q Ability
  (Rendering|SetVisibility (Variables|Default|GetAniviaQRangeIndicatorMesh) false false)
  (bind _returnvalue_2 (Game|SpawnActorfromClass "/Game/AbilitiesBP/Anivia/AniviaQ.AniviaQ_C" (Math|Transform|MakeTransform _returnvalue (Math|Rotator|MakeRotator 0.0 0.0 (.yaw (Math|Rotator|FindLookatRotation _returnvalue (Transformation|GetWorldLocation (Variables|Default|GetFlatCursor))))) "1,1,1") "Undefined" 0 0))
  (Variables|Default|SetSpawnedAniviaQ _returnvalue_2)
  (Variables|Default|SetIsSettingQ false)
  (Variables|Default|SetCanUseQ false)
  (Default|ResetCooldownSwitcher (Variables|Default|GetHUD) "NewEnumerator0")
  (Utilities|FlowControl|Delay (Variables|Default|GetQCooldown))
  (Variables|Default|SetCanUseQ true))

(event Custom|TryCancelSetQ
  ;[1 1 1] Cancel abilities without officially activating them
  (if (Variables|Default|GetIsSettingQ)
    (Variables|Default|SetIsSettingQ false)
    (Rendering|SetVisibility (Variables|Default|GetAniviaQRangeIndicatorMesh) false false)))

(event Custom|MoveInRangeOfETarget
  (bind _abilityspawnpoint (Variables|Default|GetAbilitySpawnPoint))
  (bind _returnvalue (Transformation|GetWorldTransform _abilityspawnpoint))
  ;[1 1 1] Automatically move in firing range of E target
  (bind _astop_down_controller (Utilities|Casting|CastToTopDownController (Game|GetPlayerController 0)))
  (if (Variables|/Game/TopDownBP/Blueprints/TopDownController.TopDownController_C|GetMovementInputtedThisFrame _astop_down_controller) ; Check whether autopathing towards enemy is overwritten by new movment command
    (Variables|Default|SetETarget 0)
    (Variables|Default|SetIsSettingE false)
    (Rendering|SetVisibility (Variables|Default|GetCircularAbilityRangeIndicator) false false)
    (elif (<= (Transformation|GetDistanceTo (Components|GetOwner (Variables|Default|GetETarget))) (* (Variables|Default|GetAniviaECastRange) 5e+01))
      (Components|Movement|StopMovementImmediately (Variables|Character|GetCharacterMovement)) ; Stop, as character is in range of target
      (CallFunction|SpawnandTargetEAbility (.location _returnvalue) (Math|Rotator|FindLookatRotation (.location _returnvalue) (Transformation|GetWorldLocation (Variables|Default|GetETarget))) (Variables|Default|GetETarget))
      (Variables|Default|SetETarget 0)
      (else
        (AI|Navigation|SimpleMovetoLocation (Pawn|GetController self) (Transformation|GetWorldLocation (Variables|Default|GetETarget))) ; Move in range of target
      ))))

(event Custom|TryCancelSetW
  ;[1 1 1] Cancel abilities without officially activating them
  (if (Variables|Default|GetIsSettingW)
    (Actor|DestroyActor (Variables|Default|GetSpawnedAniviaW))
    (Variables|Default|SetIsSettingW false)
    (Variables|Default|SetCanUseW true)))

(event Custom|TryCancelSetR
  ;[1 1 1] Cancel abilities without officially activating them
  (if (Variables|Default|GetIsSettingR)
    (Actor|DestroyActor (Variables|Default|GetSpawnedAniviaR))
    (Variables|Default|SetIsSettingR false)
    (Variables|Default|SetCanUseR true)))

(event Custom|TryCancelSetE
  ;[1 1 1] Cancel abilities without officially activating them
  (if (Variables|Default|GetIsSettingE)
    (Variables|Default|SetIsSettingE false)
    (Rendering|SetVisibility (Variables|Default|GetCircularAbilityRangeIndicator) false false)))

(event EventBeginPlay
  (|CallParentFunction)
  (if (Variables|Default|GetIsControllingPlayer)
    ;[1 1 1] Setup HUD
    (bind _returnvalue (UserInterface|CreateWidget "/Game/CharacterBP/Anivia/AniviaHUD.AniviaHUD_C"))
    (bind _output_get (Variables|Default|SetHUD _returnvalue))
    (Utilities|FlowControl|Sequence
      (:then_0
        (UserInterface|Viewport|AddtoViewport _output_get 0))
      (:then_1
        (Default|SetInitialCooldowns _output_get (Variables|Default|GetQCooldown) (Variables|Default|GetWCooldown) (Variables|Default|GetECooldown) (Variables|Default|GetRCooldown))))))

(event EventTick
  (params (DeltaSeconds :type Float%20%28single-precision%29))
  (bind _ismouseovermap (Variables|Default|GetIsMouseOverMap))
  (bind _returnvalue (not _ismouseovermap))
  ;[1 1 1] Event Tick
  (|CallParentFunction DeltaSeconds)
  (Utilities|FlowControl|Sequence
    (:then_0
      (if (Variables|Default|GetIsSettingW)
        (Rendering|SetActorHiddenInGame (Variables|Default|GetSpawnedAniviaW) _returnvalue)))
    (:then_1
      (if (Variables|Default|GetIsSettingR)
        (Rendering|SetActorHiddenInGame (Variables|Default|GetSpawnedAniviaR) _returnvalue)))
    (:then_2
      (if (Utilities|IsValid (Variables|Default|GetETarget))
        (CallFunction|MoveinRangeOfETarget)))
    (:then_3
      (Transformation|SetWorldRotation (Variables|Default|GetAniviaQRangePivotPoint) (Math|Rotator|MakeRotator 0.0 0.0 (.yaw (Math|Rotator|FindLookatRotation (Transformation|GetWorldLocation (Variables|Default|GetAniviaQRangePivotPoint)) (Transformation|GetWorldLocation (Variables|Default|GetFlatCursor))))) false false))))

(event Input|ActionEvents|InputActionAbilityQ
  (params (Key :type Key%20Structure))
  (bind _spawnedaniviaq (Variables|Default|GetSpawnedAniviaQ))
  ;[1 1 1] Anivia Q Ability
  (:Pressed
    (CallFunction|CancelSettingOtherAbilities "NewEnumerator0")
    (if (Variables|Default|GetCanUseQ)
      (Rendering|SetVisibility (Variables|Default|GetAniviaQRangeIndicatorMesh) true false)
      (Variables|Default|SetIsSettingQ true)
      (else
        (Utilities|IsValid _spawnedaniviaq
          (:Is%20Valid
            (if (not (Variables|/Game/AbilitiesBP/Anivia/AniviaQ.AniviaQ_C|GetHasFinishedStartAudio _spawnedaniviaq))
              (Default|StartEndAudioandPrepareDestroy _spawnedaniviaq))))))))

(event Input|ActionEvents|InputActionAbilityW
  (params (Key :type Key%20Structure))
  (bind _flatcursor (Variables|Default|GetFlatCursor))
  ;[1 1 1] Anivia W Spawn Setting Tool
  (:Pressed
    (CallFunction|CancelSettingOtherAbilities "NewEnumerator1")
    (if (Variables|Default|GetCanUseW)
      (Variables|Default|SetIsSettingW true)
      (Variables|Default|SetCanUseW false)
      (bind _returnvalue (Game|SpawnActorfromClass "/Game/AbilitiesBP/Anivia/AniviaW.AniviaW_C" (Math|Transform|MakeTransform (+ (Transformation|GetWorldLocation _flatcursor) "0, 0,8.000000") "0, 0, 0" "1,1,1") "Undefined" 0 0))
      (bind _output_get (Variables|Default|SetSpawnedAniviaW _returnvalue))
      (Transformation|AttachComponentToComponent _output_get _flatcursor "None" "KeepWorld" "KeepRelative" "KeepRelative" true))))

(event Input|ActionEvents|InputActionAcceptAction
  (params (Key :type Key%20Structure))
  (bind _spawnedaniviar (Variables|Default|GetSpawnedAniviaR))
  (bind _ismouseovermap (Variables|Default|GetIsMouseOverMap))
  (bind _abilityspawnpoint (Variables|Default|GetAbilitySpawnPoint))
  (bind _spawnedaniviaw (Variables|Default|GetSpawnedAniviaW))
  (bind _spawnedaniviaw_2 (Variables|Default|GetSpawnedAniviaW))
  (bind _mouseoverobject (Variables|Default|GetMouseOverObject))
  (bind _returnvalue (Components|GetOwner _mouseoverobject))
  (bind _returnvalue_2 (Transformation|GetWorldTransform _abilityspawnpoint))
  (bind _wallmesh (Variables|/Game/AbilitiesBP/Anivia/AniviaW.AniviaW_C|GetWallMesh _spawnedaniviaw))
  ;[1 1 1] Place abilities into world after spawn position has been decided upon
  (:Pressed
    (Utilities|FlowControl|Sequence
      (:then_0
        (if (and (Variables|Default|GetIsSettingR) _ismouseovermap)
          (Transformation|DetachFromActor _spawnedaniviar "KeepWorld" "KeepWorld" "KeepWorld")
          (Components|Activation|Activate (Variables|/Game/AbilitiesBP/Anivia/AniviaR.AniviaR_C|GetParticleSystem _spawnedaniviar) false)
          (Variables|Default|SetIsSettingR false)))
      (:then_1
        (if (and (Variables|Default|GetIsSettingW) _ismouseovermap)
          (Rendering|Material|SetMaterial _wallmesh 0 "/Game/Effects/InfinityBladeIceLands/Environments/Ice/Env_Ice_Ground/Materials/M_IceShard.M_IceShard")
          (Collision|SetCollisionEnabled _wallmesh "QueryAndPhysics")
          (Transformation|DetachFromActor _spawnedaniviaw_2 "KeepWorld" "KeepWorld" "KeepRelative")
          (Variables|/Game/AbilitiesBP/Anivia/AniviaW.AniviaW_C|SetIsPlacing _spawnedaniviaw_2 false)
          (Components|Activation|SetActive (Variables|/Game/AbilitiesBP/Anivia/AniviaW.AniviaW_C|GetStartAudio _spawnedaniviaw_2) true false)
          (Variables|Default|SetIsSettingW false)
          (Default|ResetCooldownSwitcher (Variables|Default|GetHUD) "NewEnumerator1")
          (Utilities|FlowControl|Delay (Variables|Default|GetWCooldown))
          (Variables|Default|SetCanUseW true)))
      (:then_2
        (if (Variables|Default|GetIsSettingE)
          (if (Utilities|IsValid _mouseoverobject)
            (if (!= _returnvalue self)
              (Utilities|Casting|CastToBP_TopdownParent _returnvalue)
              (if (<= (Transformation|GetDistanceTo _returnvalue) (* (Variables|Default|GetAniviaECastRange) 5e+01))
                (CallFunction|SpawnandTargetEAbility (.location _returnvalue_2) (Math|Rotator|FindLookatRotation (.location _returnvalue_2) (Transformation|GetWorldLocation _mouseoverobject)) _mouseoverobject)
                (elif true
                  (Variables|Default|SetETarget _mouseoverobject)))))))
      (:then_3
        (if (Variables|Default|GetIsSettingQ)
          (CallFunction|FireQAbility))))))

(event Input|ActionEvents|InputActionAbilityE
  (params (Key :type Key%20Structure))
  (bind _aniviaecastrange (Variables|Default|GetAniviaECastRange))
  (bind _circularabilityrangeindicator (Variables|Default|GetCircularAbilityRangeIndicator))
  ;[1 1 1] E Ability Input Handling
  (:Pressed
    (CallFunction|CancelSettingOtherAbilities "NewEnumerator2")
    (if (and (not (Variables|Default|GetIsSettingE)) (Variables|Default|GetCanUseE))
      (Variables|Default|SetIsSettingE true)
      (Transformation|SetWorldScale3D _circularabilityrangeindicator (Math|Vector|MakeVector _aniviaecastrange _aniviaecastrange 1.0))
      (Rendering|SetVisibility _circularabilityrangeindicator true false))))

(event Input|ActionEvents|InputActionCancelAction
  (params (Key :type Key%20Structure))
  ;[1 1 1] Cancel abilities without officially activating them
  (:Pressed
    (Utilities|FlowControl|Sequence
      (:then_0
        (CallFunction|TryCancelSetR))
      (:then_1
        (CallFunction|TRyCancelSetW))
      (:then_2
        (CallFunction|TryCancelSetE))
      (:then_3
        (CallFunction|TryCancelSetQ)))))

(event Input|ActionEvents|InputActionAbilityR
  (params (Key :type Key%20Structure))
  (bind _flatcursor (Variables|Default|GetFlatCursor))
  ;[1 1 1] Anivia R Spawn Setting Tool
  (:Pressed
    (CallFunction|CancelSettingOtherAbilities "NewEnumerator3")
    (if (Variables|Default|GetCanUseR)
      (Variables|Default|SetIsSettingR true)
      (Variables|Default|SetCanUseR false)
      (bind _returnvalue (Game|SpawnActorfromClass "/Game/AbilitiesBP/Anivia/AniviaR.AniviaR_C" (Math|Transform|MakeTransform (+ (Transformation|GetWorldLocation _flatcursor) "0, 0,8.000000") "0, 0, 0" "1,1,1") "Undefined" 0 0))
      (bind _output_get (Variables|Default|SetSpawnedAniviaR _returnvalue))
      (Transformation|AttachComponentToComponent _returnvalue _flatcursor "None" "KeepWorld" "KeepRelative" "KeepRelative" true)
      (elif (!= (Variables|Default|GetSpawnedAniviaR) 0)
        (if (Components|Activation|IsActive (Variables|/Game/AbilitiesBP/Anivia/AniviaR.AniviaR_C|GetParticleSystem (Variables|Default|GetSpawnedAniviaR)))
          (Actor|DestroyActor (Variables|Default|GetSpawnedAniviaR))
          (Variables|Default|SetSpawnedAniviaR 0)
          (Default|ResetCooldownSwitcher (Variables|Default|GetHUD) "NewEnumerator3")
          (Utilities|FlowControl|Delay (Variables|Default|GetRCooldown))
          (Variables|Default|SetCanUseR true))))))

(fn ConstructionScript
  (|CallParentFunction))

(fn CancelSettingOtherAbilities
  (params (NewActiveAbility :type AbilityList%20Enum :default "NewEnumerator0"))
  (Utilities|FlowControl|Sequence
    (:then_0
      (if (Utilities|Enum|NotEqual(Enum) NewActiveAbility "NewEnumerator1")
        (CallFunction|TryCancelSetW)))
    (:then_1
      (if (Utilities|Enum|NotEqual(Enum) NewActiveAbility "NewEnumerator2")
        (CallFunction|TryCancelSetE)))
    (:then_2
      (if (Utilities|Enum|NotEqual(Enum) NewActiveAbility "NewEnumerator3")
        (CallFunction|TryCancelSetR)))
    (:then_3
      (if (Utilities|Enum|NotEqual(Enum) NewActiveAbility "NewEnumerator0")
        (CallFunction|TryCancelSetQ)))))