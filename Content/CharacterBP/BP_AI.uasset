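; BP_AI is an AI character Blueprint that patrols back and forth along a straight line.
; On BeginPlay it stores its spawn location and a point 500 units ahead along its forward vector.
; Chained AIMoveTo calls send it between the two points with a short delay at each end, looping endlessly and continuing even when a move fails.
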(event EventBeginPlay
  (bind _self self)
  ;[1 1 1] Loop movment
  (Variables|Default|SetStartPosition (Transformation|GetActorLocation))
  (Variables|Default|SetForwardPosition (+ (Variables|Default|GetStartPosition) (* (Transformation|GetActorForwardVector) 5e+02)))
  (AI|AIMoveTo _self (Variables|Default|GetForwardPosition) 0 25.0 false :!label _label
    (:OnSuccess
      _)
    (:OnFail
      _))
  (Utilities|FlowControl|Delay 0.5)
  (AI|AIMoveTo _self (Variables|Default|GetStartPosition) 0 25.0 false
    (:OnSuccess
      _)
    (:OnFail
      _))
  (Utilities|FlowControl|Delay 0.5)
  (goto _label))

(fn ConstructionScript
  (|CallParentFunction))